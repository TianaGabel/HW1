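; BP_spiketrap is a one-shot spike trap triggered when the first-person player character overlaps its box.
; Until triggered, Tick calls play on the looping idle animation every frame.
; The first player overlap, gated by DoOnce, sets TrapUp, plays the damage animation once and sets the skeleton's relative rotation.
; Damage is only a debug print, and nothing resets the trap.
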(event `self.ReceiveTick`
  (params (DeltaSeconds :type "Float (single-precision)"))
  ;[1 1 1] Animations
  (if (not (`self.TrapUp`))
    (`SkeletalMeshComponent.PlayAnimation` (`self.Trap_skeleton`) "/Game/CustomBlueprints/Spike_trap/SpikeTrap_Idle_Animation.SpikeTrap_Idle_Animation" true)))

(event `self.Box.OnComponentBeginOverlap`
  (params (OverlappedComponent :type "PrimitiveComponent Object Reference") (OtherActor :type "Actor Object Reference") (OtherComp :type "PrimitiveComponent Object Reference") (OtherBodyIndex :type Integer) (bFromSweep :type Boolean) (SweepResult :type "HitResult Structure (by ref)"))
  ;[1 1 1] Animations
  (cast `/Game/FirstPerson/Blueprints/BP_FirstPersonCharacter` OtherActor)
  (`/Engine/EditorBlueprintResources/StandardMacros.DoOnce` false
    (:`Completed`
      (set `self.TrapUp` true)
      (`SkeletalMeshComponent.PlayAnimation` (`self.Trap_skeleton`) "/Game/CustomBlueprints/Spike_trap/SpikeTrap_DamageAnimation_Anim.SpikeTrap_DamageAnimation_Anim" false)
      (`SceneComponent.K2_SetRelativeRotation` (`self.Trap_skeleton`) (struct :`Roll` 90.0) false false)
      (`KismetSystemLibrary.PrintString` "Deal damage to player"))))

(fn `UserConstructionScript`)