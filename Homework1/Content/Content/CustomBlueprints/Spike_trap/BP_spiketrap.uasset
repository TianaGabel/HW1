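; BP_spiketrap is a spike trap that damages the first-person character when they step into its Box trigger.
; A DoOnce-gated overlap sets TrapUp, plays the damage animation and directly subtracts DamageAmount from the character's Health.
; Any end overlap starts a delayed reset animation, then clears TrapUp and re-arms the trap.
; While TrapUp is false, Tick replays the idle animation every frame and reasserts the skeleton's rotation.
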(event `self.ReceiveTick`
  (params (DeltaSeconds :type "Float (single-precision)"))
  (bind _trap_skeleton (`self.Trap_skeleton`))
  ;[1 1 1] Animations
  (if (not (`self.TrapUp`))
    (`SkeletalMeshComponent.PlayAnimation` _trap_skeleton "/Game/Content/CustomBlueprints/Spike_trap/SpikeTrap_Idle_Animation.SpikeTrap_Idle_Animation" true)
    (`SceneComponent.K2_SetRelativeRotation` _trap_skeleton (struct :`Roll` 90.0) false false)))

(event `self.Box.OnComponentBeginOverlap`
  (params (OverlappedComponent :type "PrimitiveComponent Object Reference") (OtherActor :type "Actor Object Reference") (OtherComp :type "PrimitiveComponent Object Reference") (OtherBodyIndex :type Integer) (bFromSweep :type Boolean) (SweepResult :type "HitResult Structure (by ref)"))
  ;[1 1 1] Animations
  (bind _asbp_first_person_character (cast `/Game/FirstPerson/Blueprints/BP_FirstPersonCharacter` OtherActor))
  (`/Engine/EditorBlueprintResources/StandardMacros.DoOnce` false :!label _label
    (:`Completed`
      (set `self.TrapUp` true)
      (`SkeletalMeshComponent.PlayAnimation` (`self.Trap_skeleton`) "/Game/Content/CustomBlueprints/Spike_trap/SpikeTrap_DamageAnimation_Anim.SpikeTrap_DamageAnimation_Anim" false)
      (`SceneComponent.K2_SetRelativeRotation` (`self.Trap_skeleton`) (struct :`Roll` 90.0) false false)
      ;[1 1 1] Deal Damage
      (set `/Game/FirstPerson/Blueprints/BP_FirstPersonCharacter.Health` (- (`/Game/FirstPerson/Blueprints/BP_FirstPersonCharacter.Health` _asbp_first_person_character) (`self.Damage Amount`)) _asbp_first_person_character))))

(event `self.Box.OnComponentEndOverlap`
  (params (OverlappedComponent :type "PrimitiveComponent Object Reference") (OtherActor :type "Actor Object Reference") (OtherComp :type "PrimitiveComponent Object Reference") (OtherBodyIndex :type Integer))
  ;[1 1 1] Animations
  (`KismetSystemLibrary.Delay` 5.0)
  (`SkeletalMeshComponent.PlayAnimation` (`self.Trap_skeleton`) "/Game/Content/CustomBlueprints/Spike_trap/SpikeTrap_ResetAnimation_Anim1.SpikeTrap_ResetAnimation_Anim1" false)
  (`KismetSystemLibrary.Delay` 2.0)
  (set `self.TrapUp` false)
  (`SceneComponent.K2_SetRelativeRotation` (`self.Trap_skeleton`) (struct :`Roll` 90.0) false false)
  (goto _label :!via `Reset`))

(fn `UserConstructionScript`)